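; VR pawn for a ball-catching game, handling calibration of the hand controller origin against the BallCatcherManager.
; Right trigger repositions the manager's cylinder, and Tick can keep a running average of the right controller's position while aggregation is enabled.
; SetControllerOrigin stops averaging, offsets HandsOrigin to align that average with the manager's starting position, and moves the cylinder again.
; The nodes that reset and enable averaging are unconnected.
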(event Custom|Set%20Controller%20Origin
  (bind _handsorigin (Variables|Default|GetHandsOrigin))
  (Development|PrintString "Done Calibarting")
  (Variables|Default|SetbAggregateAveragePosition false)
  (Transformation|SetWorldLocation _handsorigin (+ (Transformation|GetWorldLocation _handsorigin) (- (Transformation|GetWorldLocation (Variables|/Script/RobotControl.ObjectCatcherManager|GetControllerStartingPosition (Variables|Default|GetBallCatcherManager))) (Variables|Default|GetAverageControllerPosition))) false false)
  (Transformation|SetWorldLocation (Variables|/Game/Actors/BP_ObjectCatcherManager.BP_ObjectCatcherManager_C|GetCylinder (Variables|Default|GetBallCatcherManager)) (Math|Vector|MakeVector -2.3e+02 0.0 -35.0) false false))

(event EventBeginPlay
  (|CallParentFunction)
  (Variables|Default|SetAverageControllerPosition (Transformation|GetWorldLocation (Variables|Default|GetRightController))))

(event Collision|EventActorBeginOverlap
  (params (OtherActor :type Actor%20Object%20Reference)))

(event EventTick
  (params (DeltaSeconds :type Float%20%28single-precision%29))
  (|CallParentFunction DeltaSeconds)
  (if (Variables|Default|GetbAggregateAveragePosition)
    (Variables|Default|SetAverageControllerPosition (|((OldAverage*((n-1)/n))+(NewSample/n)) (Variables|Default|GetAverageControllerPosition) (Math|Conversions|ToFloat(Integer) (Variables|Default|GetAverageWeight)) (Transformation|GetWorldLocation (Variables|Default|GetRightController))))
    (Math|Integer|IncrementInt (Variables|Default|GetAverageWeight))))

(event Input|KeyboardEvents|MotionControllerRightTrigger
  (params (Key :type Key%20Structure :default "None"))
  (:Pressed
    (Development|PrintString "Calibrating")
    (Transformation|SetRelativeLocation (Variables|/Game/Actors/BP_ObjectCatcherManager.BP_ObjectCatcherManager_C|GetCylinder (Variables|Default|GetBallCatcherManager)) "0, 0,5.000000" false false)))

(fn ConstructionScript)