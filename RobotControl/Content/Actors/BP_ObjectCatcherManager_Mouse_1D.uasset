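; Object catcher manager, apparently the one-axis mouse variant, that moves a Cylinder catcher along X in a falling-ball catching task.
; Tick adds an input axis value, scaled by delta time and Speed, to the cylinder's relative X and pins Z to a constant.
; GetCatcherToBallDistance returns the absolute world X gap between cylinder and CurrentFallingBall.
; A VR-controller movement chain is left unconnected, and TestButton only prints a debug message.
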(event `self.ReceiveBeginPlay`)

(event `InputAction|TestButton`
  (params (Key :type "Key Structure"))
  (:`Pressed`
    (`KismetSystemLibrary.PrintString` "TEST HAS BEEN PRESSED!")))

(event `self.ReceiveTick`
  (params (DeltaSeconds :type "Float (single-precision)"))
  (bind _cylinder (`self.Cylinder`))
  (`SceneComponent.K2_SetRelativeLocation` _cylinder (`KismetMathLibrary.MakeVector` (+ (.x (`SceneComponent.RelativeLocation` _cylinder)) (* (* (`self.GetInputAxisKeyValue`) DeltaSeconds) (`self.Speed`))) 0.0 5.0) false false))

(fn `GetCatcherToBallDistance`
  (returns (ReturnValue :type "Float (double-precision)"))
  (bind _returnvalue_x (`KismetMathLibrary.BreakVector` (- (`SceneComponent.K2_GetComponentLocation` (`self.Cylinder`)) (`SceneComponent.K2_GetComponentLocation` (`BallToCatch.StaticMesh` (`self.CurrentFallingBall`))))))
  (return (`KismetMathLibrary.Abs` _returnvalue_x)))

(fn `UserConstructionScript`)