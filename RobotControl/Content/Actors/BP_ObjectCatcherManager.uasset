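; BP_ObjectCatcherManager moves a Cylinder, presumably the object catcher, along a fixed low height using the player pawn's right motion controller.
; On BeginPlay, the cylinder snaps to the controller's world X and Y.
; Each tick, it adds the controller's relative-position delta, rotated by the camera's world rotation, to the cylinder's horizontal position, then stores that relative position for the next frame.
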(event `self.ReceiveBeginPlay`
  (bind (_returnvalue_x _returnvalue_y) (`KismetMathLibrary.BreakVector` (`SceneComponent.K2_GetComponentLocation` (`VR_Pawn.RightController` (`self.PlayerPawn`)))))
  (`SceneComponent.K2_SetWorldLocation` (`self.Cylinder`) (`KismetMathLibrary.MakeVector` _returnvalue_x _returnvalue_y 5.0) false false))

(event `self.ReceiveTick`
  (params (DeltaSeconds :type "Float (single-precision)"))
  (bind _relativelocation (`SceneComponent.RelativeLocation` (`VR_Pawn.RightController` (`self.PlayerPawn`))))
  (bind (_returnvalue_x _returnvalue_y) (`KismetMathLibrary.BreakVector` (+ (`KismetMathLibrary.GreaterGreater_VectorRotator` (- _relativelocation (`self.RightControllerPreviousRelativePosition`)) (`SceneComponent.K2_GetComponentRotation` (`VR_Pawn.Camera` (`self.PlayerPawn`)))) (`SceneComponent.K2_GetComponentLocation` (`self.Cylinder`)))))
  (`SceneComponent.K2_SetWorldLocation` (`self.Cylinder`) (`KismetMathLibrary.MakeVector` _returnvalue_x _returnvalue_y 5.0) false false)
  (set `self.RightControllerPreviousRelativePosition` _relativelocation))

(fn `UserConstructionScript`)