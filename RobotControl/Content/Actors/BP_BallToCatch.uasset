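; BP_BallToCatch is a ball in an object-catching game that reports to its ManagerObject whether it was caught or fell.
; A mesh overlap with a BP_ObjectCatcherManager actor, before any fall, calls OnBallCaught and destroys the ball at once.
; The first mesh hit latches AlreadyFell, blocking later catches, then calls OnBallFell and destroys the ball after a short delay.
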(event `self.StaticMesh.OnComponentHit`
  (params (HitComponent :type "PrimitiveComponent Object Reference") (OtherActor :type "Actor Object Reference") (OtherComp :type "PrimitiveComponent Object Reference") (NormalImpulse :type "Vector Structure") (Hit :type "HitResult Structure (by ref)"))
  (if (not (`self.bAlreadyFell`))
    (set `self.bAlreadyFell` true)
    (`ObjectCatcherManager.OnBallFell` (`self.ManagerObject`))
    (`KismetSystemLibrary.Delay` 1.0)
    (`self.K2_DestroyActor`)))

(event `self.StaticMesh.OnComponentBeginOverlap`
  (params (OverlappedComponent :type "PrimitiveComponent Object Reference") (OtherActor :type "Actor Object Reference") (OtherComp :type "PrimitiveComponent Object Reference") (OtherBodyIndex :type Integer) (bFromSweep :type Boolean) (SweepResult :type "HitResult Structure (by ref)"))
  (if (and (== (`GameplayStatics.GetObjectClass` OtherActor) "/Game/Actors/BP_ObjectCatcherManager.BP_ObjectCatcherManager_C") (not (`self.bAlreadyFell`)))
    (`ObjectCatcherManager.OnBallCaught` (`self.ManagerObject`))
    (`self.K2_DestroyActor`)))

(fn `UserConstructionScript`)