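; BP_ObjectCatcherManager_Mouse_2D is an actor that slides a Cylinder, apparently a mouse-driven object catcher, across a flat plane.
; Each Tick adds axis key input scaled by delta time and Speed to the Cylinder's relative X and Y, holding Z fixed.
; A TestButton press only prints a debug message.
; An unconnected leftover would instead position the Cylinder from the player pawn's right controller and camera rotation.
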(event `self.ReceiveBeginPlay`)

(event `InputAction|TestButton`
  (params (Key :type "Key Structure"))
  (:`Pressed`
    (`KismetSystemLibrary.PrintString` "TEST HAS BEEN PRESSED!")))

(event `self.ReceiveTick`
  (params (DeltaSeconds :type "Float (single-precision)"))
  (bind _cylinder (`self.Cylinder`))
  (bind _speed (`self.Speed`))
  (`SceneComponent.K2_SetRelativeLocation` _cylinder (`KismetMathLibrary.MakeVector` (+ (.x (`SceneComponent.RelativeLocation` _cylinder)) (* (* (`self.GetInputAxisKeyValue`) DeltaSeconds) _speed)) (+ (.y (`SceneComponent.RelativeLocation` _cylinder)) (* (* (`self.GetInputAxisKeyValue`) DeltaSeconds) _speed)) 5.0) false false))

(fn `UserConstructionScript`)